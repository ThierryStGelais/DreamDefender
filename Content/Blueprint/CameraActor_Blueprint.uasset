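; Fixed-position camera actor that becomes the player's view target and carries a glowstick counter and transition picture.
; Construction sets its transform and gives four glowstick meshes dynamic materials, which UpdateGlowStickNumber lights through an emissive parameter according to the count.
; Other functions toggle glowstick visibility and show a transition sprite with the game paused, or hide it.
; BeginPlay retries until the ThirdPersonCharacter exists; the older text counter stays hidden.
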(event EventBeginPlay
  (bind _asthird_person_character (Utilities|Casting|CastToThirdPersonCharacter (Game|GetPlayerCharacter 0) :!label _label)
    (:then
      (Utilities|FlowControl|Sequence
        (:then_0
          (bind _returnvalue (Utilities|Casting|CastToPlayerController (Game|GetPlayerController 0)))
          (Game|Player|SetViewTargetwithBlend _returnvalue self 0.0 "VTBlend_Linear" 0.0 false)
          ;[1 1 1] Texte invisible au depart
          (Rendering|Components|TextRender|SetText (Variables|Default|GetGlowstickNumberText) (Utilities|Text|ToText(Integer) (Variables|Default|GetGlowstick_Number) false))
          (Rendering|SetVisibility (Variables|Default|GetGlowstickNumberText) false false))))
    (:CastFailed
      (Utilities|FlowControl|Delay 0 0.005)
      (goto _label))))

(event EventTick
  (params (DeltaSeconds :type Float%20%28single-precision%29))
  ;[1 0 0] What kind of madness was this ?
)

(fn ConstructionScript
  ;[1 1 1] Set camera location/rotation
  (Transformation|SetActorLocationAndRotation "-1560.000000,-122.000000,410.000000" "-25.000000, 0, 0")
  (Utilities|FlowControl|Sequence
    (:then_0
      (bind _returnvalue (Rendering|Material|CreateDynamicMaterialInstance (Variables|Default|GetGlowStick1) 0 "/Game/Material/Level_Design/MAT_GlowStick_Ground_Inst.MAT_GlowStick_Ground_Inst" :!class /Script/Engine.PrimitiveComponent))
      (Rendering|Material|SetScalarParameterValue _returnvalue "IsGreenEmissive" 0.0 :!class /Script/Engine.MaterialInstanceDynamic))
    (:then_1
      (bind _returnvalue_2 (Rendering|Material|CreateDynamicMaterialInstance (Variables|Default|GetGlowStick2) 0 "/Game/Material/Level_Design/MAT_GlowStick_Ground_Inst.MAT_GlowStick_Ground_Inst" :!class /Script/Engine.PrimitiveComponent))
      (Rendering|Material|SetScalarParameterValue _returnvalue_2 "IsGreenEmissive" 0.0 :!class /Script/Engine.MaterialInstanceDynamic))
    (:then_2
      (bind _returnvalue_3 (Rendering|Material|CreateDynamicMaterialInstance (Variables|Default|GetGlowStick3) 0 "/Game/Material/Level_Design/MAT_GlowStick_Ground_Inst.MAT_GlowStick_Ground_Inst" :!class /Script/Engine.PrimitiveComponent))
      (Rendering|Material|SetScalarParameterValue _returnvalue_3 "IsGreenEmissive" 0.0 :!class /Script/Engine.MaterialInstanceDynamic))
    (:then_3
      (bind _returnvalue_4 (Rendering|Material|CreateDynamicMaterialInstance (Variables|Default|GetGlowStick4) 0 "/Game/Material/Level_Design/MAT_GlowStick_Ground_Inst.MAT_GlowStick_Ground_Inst" :!class /Script/Engine.PrimitiveComponent))
      (Rendering|Material|SetScalarParameterValue _returnvalue_4 "IsGreenEmissive" 0.0 :!class /Script/Engine.MaterialInstanceDynamic))))

(fn ResetTransition
  (Rendering|SetVisibility (Variables|Transition|GetTransitionPicture) false false))

(fn PlayTransition
  (params (Transition%20Sprite :type Paper%20Sprite%20Object%20Reference))
  (bind _transitionpicture (Variables|Transition|GetTransitionPicture))
  (Game|SetGamePaused 0 false)
  (Rendering|Components|Sprite|SetSprite _transitionpicture Transition%20Sprite)
  (Rendering|SetVisibility _transitionpicture true false)
  (Game|SetGamePaused 0 true))

(fn UpdateGlowStickNumber
  (params (GlowStickNumber :type Integer))
  ;[1 1 1] Update glowsticks
  (bind _output_get (LocalVariables|SetCurrentGlowStickNumber GlowStickNumber))
  (LocalVariables|SetMin1 (> _output_get 0))
  (LocalVariables|SetMin2 (> _output_get 1))
  (LocalVariables|SetMin3 (> _output_get 2))
  (LocalVariables|SetMin4 (> _output_get 3))
  (Utilities|FlowControl|Sequence
    (:then_0
      (bind _asmaterial_instance_dynamic (Utilities|Casting|CastToMaterialInstanceDynamic (Rendering|Material|GetMaterial (Variables|Default|GetGlowStick1) 0)))
      (if (LocalVariables|GetMin1)
        (Rendering|Material|SetScalarParameterValue _asmaterial_instance_dynamic "IsGreenEmissive" 1.0 :!class /Script/Engine.MaterialInstanceDynamic)
        (else
          (Rendering|Material|SetScalarParameterValue _asmaterial_instance_dynamic "IsGreenEmissive" 0.0 :!class /Script/Engine.MaterialInstanceDynamic))))
    (:then_1
      (bind _asmaterial_instance_dynamic_2 (Utilities|Casting|CastToMaterialInstanceDynamic (Rendering|Material|GetMaterial (Variables|Default|GetGlowStick2) 0)))
      (if (LocalVariables|GetMin2)
        (Rendering|Material|SetScalarParameterValue _asmaterial_instance_dynamic_2 "IsGreenEmissive" 1.0 :!class /Script/Engine.MaterialInstanceDynamic)
        (else
          (Rendering|Material|SetScalarParameterValue _asmaterial_instance_dynamic_2 "IsGreenEmissive" 0.0 :!class /Script/Engine.MaterialInstanceDynamic))))
    (:then_2
      (bind _asmaterial_instance_dynamic_3 (Utilities|Casting|CastToMaterialInstanceDynamic (Rendering|Material|GetMaterial (Variables|Default|GetGlowStick3) 0)))
      (if (LocalVariables|GetMin3)
        (Rendering|Material|SetScalarParameterValue _asmaterial_instance_dynamic_3 "IsGreenEmissive" 1.0 :!class /Script/Engine.MaterialInstanceDynamic)
        (else
          (Rendering|Material|SetScalarParameterValue _asmaterial_instance_dynamic_3 "IsGreenEmissive" 0.0 :!class /Script/Engine.MaterialInstanceDynamic))))
    (:then_3
      (bind _asmaterial_instance_dynamic_4 (Utilities|Casting|CastToMaterialInstanceDynamic (Rendering|Material|GetMaterial (Variables|Default|GetGlowStick4) 0)))
      (if (LocalVariables|GetMin4)
        (Rendering|Material|SetScalarParameterValue _asmaterial_instance_dynamic_4 "IsGreenEmissive" 1.0 :!class /Script/Engine.MaterialInstanceDynamic)
        (else
          (Rendering|Material|SetScalarParameterValue _asmaterial_instance_dynamic_4 "IsGreenEmissive" 0.0 :!class /Script/Engine.MaterialInstanceDynamic))))))

(fn ToggleGlowStickVisibility
  (if (Variables|/Script/Engine.SceneComponent|GetbVisible (Variables|Default|GetGlowStick1))
    (Utilities|FlowControl|Sequence
      (:then_0
        (Rendering|SetVisibility (Variables|Default|GetGlowStick1) false false))
      (:then_1
        (Rendering|SetVisibility (Variables|Default|GetGlowStick2) false false))
      (:then_2
        (Rendering|SetVisibility (Variables|Default|GetGlowStick3) false false))
      (:then_3
        (Rendering|SetVisibility (Variables|Default|GetGlowStick4) false false)))
    (else
      (Utilities|FlowControl|Sequence
        (:then_0
          (Rendering|SetVisibility (Variables|Default|GetGlowStick1) true false))
        (:then_1
          (Rendering|SetVisibility (Variables|Default|GetGlowStick2) true false))
        (:then_2
          (Rendering|SetVisibility (Variables|Default|GetGlowStick3) true false))
        (:then_3
          (Rendering|SetVisibility (Variables|Default|GetGlowStick4) true false))))))