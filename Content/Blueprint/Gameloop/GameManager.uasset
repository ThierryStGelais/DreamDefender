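; Game instance-style manager that handles level flow and progress saving, switching between main menu, numbered play levels and end-game credits.
; Advancing increments the level index, saves it to a SaveGameData slot, then opens the next PlayLevels entry or returns to the menu after the last.
; Init creates the save object and calls LoadGame, whose self-comparison check always takes the failure branch, so saved progress is never restored.
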(event EventInit
  (SaveGame|InitializeSaveGame)
  (SaveGame|LoadGame))

(fn SwitchScene
  (params (Level :type SceneList%20Enum))
  (switch Utilities|FlowControl|Switch|SwitchonSceneList Level
    (:NewEnumerator0
      (Game|OpenLevel(byName) 0 "MainMenu"))
    (:NewEnumerator1
      (LevelSwitch|GotoNextLevel))
    (:NewEnumerator2
      (Game|OpenLevel(byName) 0 "EndGameCredits"))))

(fn SwitchPlayLevel
  (params (level%20number :type Integer))
  (bind _playlevels (Variables|LevelSwitch|GetPlayLevels))
  (bind _item (Utilities|Array|Get(acopy) _playlevels level%20number))
  (Variables|LevelSwitch|SetCurrentPlayLevel level%20number)
  (Game|OpenLevel(byName) 0 _item)
  (bind _asgame_mode_dd (Utilities|Casting|CastToGameModeDD (Game|GetGameMode)))
  (Default|EventonStart _asgame_mode_dd)
  (Development|PrintString 0 (Utilities|String|ToString(Name) _item) false))

(fn GotoNextLevel
  (bind _result (Math|Integer|IncrementInt (Variables|LevelSwitch|GetCurrentPlayLevel))
    (:%20%20
      (SaveGame|SaveGame)
      (if (LevelSwitch|CheckCompletedAllLevel)
        (LevelSwitch|SwitchScene "NewEnumerator0")
        (else
          (LevelSwitch|SwitchPlayLevel _result))))))

(fn GetCurrentPlayLevel
  (return (Variables|LevelSwitch|GetCurrentPlayLevel)))

(fn InitializeSaveGame
  (bind _returnvalue (SaveGame|CreateSaveGameObject "/Game/Blueprint/Gameloop/SaveGameData.SaveGameData_C"))
  (bind _assave_game_data (Utilities|Casting|CastToSaveGameData _returnvalue))
  (Variables|SaveGame|SetSavedGameData _assave_game_data))

(fn LoadGame
  (bind _returnvalue (SaveGame|LoadGamefromSlot (Variables|/Game/Blueprint/Gameloop/SaveGameData.SaveGameData_C|GetFilename (Variables|SaveGame|GetSavedGameData)) (Variables|/Game/Blueprint/Gameloop/SaveGameData.SaveGameData_C|GetUserID (Variables|SaveGame|GetSavedGameData))))
  (if (not (== _returnvalue _returnvalue))
    (Development|PrintString 0 "Game Loaded" false true "(R=0.000000,G=1.000000,B=0.049290,A=1.000000)")
    (bind _assave_game_data (Utilities|Casting|CastToSaveGameData _returnvalue))
    (bind _output_get (Variables|SaveGame|SetSavedGameData _assave_game_data))
    (Variables|LevelSwitch|SetCurrentPlayLevel (Variables|/Game/Blueprint/Gameloop/SaveGameData.SaveGameData_C|GetcurrentLevel _output_get))
    (else
      (Development|PrintString 0 "Game Failed to load" false true "(R=1.000000,G=0.098677,B=0.000000,A=1.000000)"))))

(fn SaveGame
  (bind _savedgamedata (Variables|SaveGame|GetSavedGameData))
  (Variables|/Game/Blueprint/Gameloop/SaveGameData.SaveGameData_C|SetcurrentLevel _savedgamedata (Variables|LevelSwitch|GetCurrentPlayLevel))
  (bind _returnvalue (SaveGame|SaveGametoSlot _savedgamedata (Variables|/Game/Blueprint/Gameloop/SaveGameData.SaveGameData_C|GetFilename _savedgamedata) (Variables|/Game/Blueprint/Gameloop/SaveGameData.SaveGameData_C|GetUserID _savedgamedata)))
  (if _returnvalue
    (Development|PrintString 0 "Game Saved" false true "(R=0.251143,G=1.000000,B=0.000000,A=1.000000)")
    (else
      (Development|PrintString 0 "Game Failed to save" false true "(R=1.000000,G=0.031819,B=0.000000,A=1.000000)"))))

(fn ResetSaveGame
  (Variables|/Game/Blueprint/Gameloop/SaveGameData.SaveGameData_C|SetcurrentLevel (Variables|SaveGame|GetSavedGameData) 0))

(fn CheckCompletedAllLevel
  (return (== (Variables|LevelSwitch|GetCurrentPlayLevel) (Utilities|Array|Length (Variables|LevelSwitch|GetPlayLevels)))))

(fn ResetPlayLevel
  (LevelSwitch|SwitchPlayLevel (Variables|LevelSwitch|GetCurrentPlayLevel)))

(fn IsatLastPlayLevel
  (return (== (- (Utilities|Array|Length (Variables|LevelSwitch|GetPlayLevels)) 1) (Variables|LevelSwitch|GetCurrentPlayLevel))))