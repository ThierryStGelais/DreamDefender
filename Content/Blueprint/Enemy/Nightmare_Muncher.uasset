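; Nightmare_Muncher is an enemy Blueprint that builds on a parent class and reacts to light damage.
; Its construction script creates a dynamic creep material instance on the mesh and initialises the health-driven effect parameter.
; Transparency updates run the parent logic, then flag the Blackboard that it is being attacked.
; On EndPlay it asks GameModeDD to clear its muncher ripples.
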(event Custom|TakeDamage
  (AI|Components|Blackboard|SetValueasBool (AI|GetBlackboard 0) (Variables|Default|GetisBeingAttacked) true))

(event EventBeginPlay)

(event EventEndPlay
  (params (EndPlayReason :type EEndPlayReason%20Enum :default "Destroyed"))
  (bind _asgame_mode_dd (Utilities|Casting|CastToGameModeDD (Game|GetGameMode)))
  (Default|ClearRippleMunchers _asgame_mode_dd self))

(event EventUpdateTransparency
  (params (lightDamageFrequency :type Float%20%28single-precision%29))
  (|CallParentFunction lightDamageFrequency)
  (CallFunction|TakeDamage))

(fn ConstructionScript
  (|CallParentFunction)
  (bind _returnvalue (Rendering|Material|CreateDynamicMaterialInstance (Variables|Character|GetMesh) 0 "/Game/Material/M_Creep_CTRL.M_Creep_CTRL" :!class /Script/Engine.PrimitiveComponent))
  (Variables|Default|SetDynamicMat _returnvalue)
  (Rendering|Material|SetScalarParameterValue (Variables|Default|GetDynamicMat) "Health (200-0)" (Variables|Default|GetBaseMatEffect) :!class /Script/Engine.MaterialInstanceDynamic)
  (Variables|Default|SetLastEffectValue 2e+02))