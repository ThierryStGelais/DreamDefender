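; Base class for Nightmare enemies, which react visually to light damage and handle their own death.
; UpdateTransparency maps health to five effect steps, blends a dynamic material parameter via timeline, and swaps idle particles for damage particles until Tick detects light damage has stopped.
; Die plays death effects and camera shake, then notifies GameModeDD and destroys the actor after a delay.
; On destruction, overlapping flashlights that cannot boost gain kill streak.
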(event EventBeginPlay
  (Components|Activation|Activate (Variables|Default|GetP_Dark_Damage) false)
  (Effects|Components|ParticleSystem|SetEmitterEnable (Variables|Default|GetP_Dark_Damage) "DamageEmitter" false))

(event EventActorBeginOverlap
  (params (OtherActor :type Actor%20Object%20Reference)))

(event EventTick
  (params (DeltaSeconds :type Float%20%28single-precision%29))
  ;[1 1 1] Dans l'event tick je prend le temps depuis le dernier dégât et je l'update.Si le temps est supérieur à la fréquence de degat de la lumière, alors le nightmare est illuminé. Si le nightmare est illuminé, on reset son emitter idle et on enleve l'emitter de degats.
  (bind _output_get (Variables|Default|SetTimeSinceLastDamage (+ DeltaSeconds (Variables|Default|GetTimeSinceLastDamage))))
  (if (Variables|Default|GetisIlluminated)
    (if (> _output_get (+ (stale EventUpdateTransparency lightDamageFrequency) 0.1))
      (Variables|Default|SetisIlluminated false)
      (Effects|Components|ParticleSystem|SetEmitterEnable (Variables|Default|GetIdle%20Particle) "Idle" true)
      (Effects|Components|ParticleSystem|SetEmitterEnable (Variables|Default|GetP_Dark_Damage) "DamageEmitter" false))))

(event EventUpdateTransparency
  (params (lightDamageFrequency :type Float%20%28single-precision%29))
  ;[1 1 1] Update du monstre quand il se prend du dégât
  (Effects|Components|ParticleSystem|SetEmitterEnable (Variables|Default|GetIdle%20Particle) "Idle" false)
  (Effects|Components|ParticleSystem|SetEmitterEnable (Variables|Default|GetP_Dark_Damage) "DamageEmitter" true)
  (bind _returnvalue (Class|NightmareBaseClass|GetCurrentHealth))
  (bind _effect_value (CallFunction|GetEffectValue (/ _returnvalue (Variables|Default|GetfBaseHealth))))
  (bind _value (Timeline|Value Play)
    (:Update
      (Rendering|Material|SetScalarParameterValue (Variables|Default|GetDynamicMat) "Health (200-0)" (Math|Float|Lerp (Variables|Default|GetLastEffectValue) _effect_value _value) :!class /Script/Engine.MaterialInstanceDynamic)
      (Variables|Default|SetLastEffectValue _effect_value)
      (Variables|Default|SetTimeSinceLastDamage 0.0)
      (Variables|Default|SetisIlluminated true))))

(event EventDie
  ;[1 1 1] Evenènement de mort d'un nightmare
  (if (not (Variables|Default|GetisDead))
    (Variables|Default|SetisDead true)
    (Audio|SpawnSoundatLocation 0 (Variables|/Script/Engine.AudioComponent|GetSound (Variables|Default|GetDeathSound)) (Transformation|GetActorLocation self))
    (Utilities|FlowControl|Sequence
      (:then_0
        ;;[1 1 1] ON REND LE MESH INVISIBLE
        (Rendering|SetVisibility (Variables|Character|GetMesh) false true))
      (:then_1
        ;;[1 1 1] ON SHAKE LA CAMÉRA
        (Class|PlayerCameraManager|PlayCameraShake (Game|GetPlayerCameraManager 0) "/Game/Blueprint/Camera_shake.Camera_shake_C" 1.0 "CameraLocal" "0, 0, 0"))
      (:then_2
        ;;[1 1 1] ON SPAWN L'EMITTEUR DE PARTICULES DE MORT
        (Effects|SpawnEmitteratLocation 0 "/Game/Particles/P_Dark_Death.P_Dark_Death" (Transformation|GetActorLocation)))
      (:then_3
        ;;[1 1 1] ON MET A OFF L'EMITTEUR DE PARTICULES IDLE DE L'ENNEMI
        (Rendering|SetVisibility (Variables|Default|GetIdle%20Particle) false false)
        (Rendering|SetVisibility (Variables|Character|GetMesh) false false))
      (:then_4)
      (:then_5
        ;;[1 1 1] ON DÉTRUIT L'ACTEUR
        (Utilities|FlowControl|Delay 0 0.3)
        (bind _asgame_mode_dd (Utilities|Casting|CastToGameModeDD (Game|GetGameMode))
          (:then
            (Default|IncrementDeadEnemy _asgame_mode_dd))
          (:CastFailed
            _))
        (Actor|DestroyActor)))))

(event EventDestroyed
  (for _array_element (Collision|GetOverlappingActors "/Game/Blueprint/Light/BPLight_FlashLight.BPLight_FlashLight_C" :!class /Script/Engine.Actor)
    (bind _asbplight_flash_light (Utilities|Casting|CastToBPLight_FlashLight _array_element))
    (if (not (Variables|/Game/Blueprint/Light/BPLight_FlashLight.BPLight_FlashLight_C|GetCanBoost _asbplight_flash_light))
      (Math|Integer|IncrementInt (Variables|/Game/Blueprint/Light/BPLight_FlashLight.BPLight_FlashLight_C|GetKillStreak _asbplight_flash_light)))))

(fn ConstructionScript
  (CallFunction|SetUpStats))

(fn SetUpStats
  (bind _charactermovement (Variables|Character|GetCharacterMovement))
  (Variables|/Script/Engine.CharacterMovementComponent|SetMaxWalkSpeed _charactermovement (Variables|Stats|GetMouvementSpeed))
  (Variables|/Script/Engine.CharacterMovementComponent|SetMaxAcceleration _charactermovement (Variables|Stats|GetAcceleration)))

(fn GetEffectValue
  (params (HealthPercentage :type Float%20%28single-precision%29))
  (if (>= HealthPercentage 0.8)
    (LocalVariables|SetReturnValue (Utilities|Array|Get(acopy) (LocalVariables|GetEffect%20value%20Array)))
    (elif (>= HealthPercentage 0.6)
      (LocalVariables|SetReturnValue (Utilities|Array|Get(acopy) (LocalVariables|GetEffect%20value%20Array) 1))
      (elif (>= HealthPercentage 0.4)
        (LocalVariables|SetReturnValue (Utilities|Array|Get(acopy) (LocalVariables|GetEffect%20value%20Array) 2))
        (elif (>= HealthPercentage 0.2)
          (LocalVariables|SetReturnValue (Utilities|Array|Get(acopy) (LocalVariables|GetEffect%20value%20Array) 3))
          (else
            (LocalVariables|SetReturnValue (Utilities|Array|Get(acopy) (LocalVariables|GetEffect%20value%20Array) 4)))))))
  (return (LocalVariables|GetReturnValue)))