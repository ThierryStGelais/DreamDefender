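; Base light actor that detects Nightmare enemies in a cone or sphere of light, with configurable damage.
; A query-only mesh serves as the hit volume, and its scaled bounds size the matching spot or point light.
; BeginPlay registers already-overlapping Nightmares and loops EnemiesInLightUpdate on a timer set by the damage interval.
; Hit events play separate Creep or Muncher sounds, with exit binding stops to audio completion.
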(event Custom|OnAudioFinished_Event_0
  (Audio|Components|Audio|Stop (Variables|Default|GetCreepOnHit)))

(event Custom|UpdateEvent
  (Class|BaseLight|EnemiesinLightUpdate))

(event Custom|OnAudioFinished_Event_1
  (Audio|Components|Audio|Stop (Variables|Default|GetMuncherOnHit)))

(event EventBeginPlay
  (bind _returnvalue (Class|BaseLight|GetDamageTime))
  (Utilities|Time|SetTimerbyEvent (delegate Custom|UpdateEvent) _returnvalue true)
  (bind _array_element (Utilities|Array|ForEachLoopwithBreak (Collision|GetOverlappingActors 0 :!class /Script/Engine.Actor))
    (:LoopBody
      (bind _asnightmare_base_class (Utilities|Casting|CastToNightmare_BaseClass _array_element))
      (Class|BaseLight|AddEnemytoArrays _asnightmare_base_class))))

(event EventStopSoundonNightmaresExit
  (EventDispatchers|AssignOnAudioFinished (Variables|Default|GetCreepOnHit) (delegate Custom|OnAudioFinished_Event_0))
  (EventDispatchers|BindEventtoOnAudioFinished (Variables|Default|GetMuncherOnHit) (delegate Custom|OnAudioFinished_Event_1)))

(event EventPlaySoundonNightmaresHit
  (params (NightmareRef :type Actor%20Object%20Reference))
  (Utilities|Casting|CastToNightmare_Creep NightmareRef
    (:then
      (if (not (Audio|Components|Audio|IsPlaying (Variables|Default|GetCreepOnHit)))
        (Audio|Components|Audio|Play (Variables|Default|GetCreepOnHit) 0.0)))
    (:CastFailed
      (if (not (Audio|Components|Audio|IsPlaying (Variables|Default|GetMuncherOnHit)))
        (Audio|Components|Audio|Play (Variables|Default|GetMuncherOnHit) 0.0)))))

(fn ConstructionScript)

(fn InitializeLightCone
  (params (bIsOn :type Boolean) (smConeMesh :type Static%20Mesh%20Object%20Reference) (fLightIntensity :type Float%20%28single-precision%29) (fLightDamage :type Float%20%28single-precision%29) (MeshRotation :type Rotator) (MeshPosition :type Vector) (DamageFrequency :type Float%20%28single-precision%29) (LightColor :type Linear%20Color%20Structure) (ConeMeshSize :type Vector) (aObjectToIgnore :type Actor%20Object%20Reference) (ConeVisible :type Boolean) (ConeMaterial :type Material%20Object%20Reference))
  (CallFunction|InitializeHitDetection smConeMesh MeshRotation MeshPosition ConeMeshSize ConeVisible bIsOn)
  (CallFunction|InitializeLightConeSpotLight fLightDamage fLightIntensity bIsOn DamageFrequency LightColor)
  (Class|BaseLight|AddParentActortoIgnore aObjectToIgnore)
  (Rendering|Material|SetMaterial (Variables|Default|GetHitDetectionMesh) 0 ConeMaterial))

(fn InitializeLightConeSpotLight
  (params (fLight%20Damage :type Float%20%28single-precision%29) (fLightIntensity :type Float%20%28single-precision%29) (bIsOn :type Boolean) (fLightDamageFrequency :type Float%20%28single-precision%29) (lcLightColor :type Linear%20Color%20Structure))
  (bind _hitdetectionmesh (Variables|Default|GetHitDetectionMesh))
  (bind _vlightconesize (Variables|Default|GetvLightConeSize))
  (bind (_min _max) (Components|StaticMesh|GetLocalBounds _hitdetectionmesh))
  (bind (_x _y _z) (Math|Vector|BreakVector _vlightconesize))
  (bind (_x_2 _y_2 _z_2) (Math|Vector|BreakVector _min))
  (bind (_x_3 _y_3 _z_3) (Math|Vector|BreakVector _max))
  (bind _returnvalue (- _y_3 _y_2))
  (bind _returnvalue_2 (- _z_3 _z_2))
  (bind _returnvalue_3 (* _z _returnvalue_2))
  (bind _returnvalue_4 (* _returnvalue _y))
  (bind _returnvalue_5 (/ _returnvalue_4 2.0))
  (bind _returnvalue_6 (Class|KismetMathLibrary|DegAtan2 _returnvalue_5 _returnvalue_3))
  ;[1 1 1] Initialisation des stats de la lumiere
  (Rendering|SetVisibility (Variables|Default|GetSpotLight) true false)
  (Class|BaseLight|SetDamageTime fLightDamageFrequency)
  (Class|BaseLight|SetLightIntensity fLightIntensity)
  (Class|BaseLight|SetDamageValue fLight%20Damage)
  ;[1 1 1] Initialisation des propriétés de la lumiere
  (Rendering|Components|Light|SetLightColor (Variables|Default|GetSpotLight) lcLightColor true)
  (Rendering|Lighting|SetInnerConeAngle (Variables|Default|GetSpotLight) _returnvalue_6)
  (Rendering|Lighting|SetOuterConeAngle (Variables|Default|GetSpotLight) _returnvalue_6)
  (Rendering|Lighting|SetAttenuationRadius (Variables|Default|GetSpotLight) (* (- _z_3 _z_2) _z))
  (if bIsOn
    (Class|BaseLight|SetLighton)
    (else
      (Class|BaseLight|SetLightOff))))

(fn InitializeHitDetection
  (params (mesh :type Static%20Mesh%20Object%20Reference) (meshRotation :type Rotator) (MeshLocation :type Vector) (coneMeshSize :type Vector) (ConeVisible :type Boolean) (IsOn :type Boolean))
  (bind _hitdetectionmesh (Variables|Default|GetHitDetectionMesh))
  (Components|StaticMesh|SetStaticMesh _hitdetectionmesh mesh)
  (Transformation|SetRelativeLocationAndRotation _hitdetectionmesh MeshLocation meshRotation false false)
  (Development|SetHiddeninGame _hitdetectionmesh (not ConeVisible) false)
  (Transformation|SetRelativeScale3D _hitdetectionmesh coneMeshSize)
  (Variables|Default|SetvLightConeSize coneMeshSize)
  (Collision|SetCollisionEnabled _hitdetectionmesh "QueryOnly")
  (Collision|SetCollisionObjectType _hitdetectionmesh "ECC_WorldStatic")
  (Rendering|SetVisibility _hitdetectionmesh IsOn false))

(fn InitializeLightSphere
  (params (Is%20On :type Boolean) (SmSphereMesh :type Static%20Mesh%20Object%20Reference) (FLightIntensity :type Float%20%28single-precision%29) (FLightDamage :type Float%20%28single-precision%29) (Damage%20Frequency :type Float%20%28single-precision%29) (Light%20Color :type Linear%20Color%20Structure) (Mesh%20Size :type Vector) (AObjectToIgnore :type Actor%20Object%20Reference) (SphereVisible :type Boolean) (MeshPosition :type Vector) (MeshRotation :type Rotator) (Material :type Material%20Object%20Reference))
  (CallFunction|InitializeHitDetection SmSphereMesh MeshRotation MeshPosition Mesh%20Size SphereVisible Is%20On)
  (CallFunction|InitializeLightSpherePointLight FLightDamage FLightIntensity Is%20On Damage%20Frequency Light%20Color)
  (Class|BaseLight|AddParentActortoIgnore AObjectToIgnore)
  (Rendering|Material|SetMaterial (Variables|Default|GetHitDetectionMesh) 0 Material))

(fn InitializeLightSpherePointLight
  (params (FLightDamage :type Float%20%28single-precision%29) (FLightIntensity :type Float%20%28single-precision%29) (IsOn :type Boolean) (FLightDamageFrenquency :type Float%20%28single-precision%29) (LcLightColor :type Linear%20Color%20Structure))
  (bind _hitdetectionmesh (Variables|Default|GetHitDetectionMesh))
  (bind (_min _max) (Components|StaticMesh|GetLocalBounds _hitdetectionmesh))
  ;[1 1 1] Initialisation des stats de la lumiere
  (Rendering|SetVisibility (Variables|Default|GetPointLight) true false)
  (Class|BaseLight|SetDamageTime FLightDamageFrenquency)
  (Class|BaseLight|SetLightIntensity FLightIntensity)
  (Class|BaseLight|SetDamageValue FLightDamage)
  (Rendering|Components|Light|SetLightColor (Variables|Default|GetPointLight) LcLightColor true)
  (Rendering|Lighting|SetAttenuationRadius (Variables|Default|GetPointLight) (/ (* (- (.X (Math|Vector|BreakVector _max)) (.X (Math|Vector|BreakVector _min))) (.X (Math|Vector|BreakVector (Variables|Default|GetvLightConeSize)))) 2.0))
  (if IsOn
    (Class|BaseLight|SetLighton)
    (else
      (Class|BaseLight|SetLightOff)))
  ;[1 1 1] N'affichera pas le cone de lumiere pour lampe torche dans l'éditeur
  (Rendering|Lighting|SetAttenuationRadius (Variables|Default|GetSpotLight) 0.0))