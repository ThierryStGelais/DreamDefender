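; Flashlight Blueprint that tracks a kill streak through IncrementKillCount and drafts a damage boost earned by streaks.
; The boost logic would enlarge the hit detection mesh, brighten the spotlight and set boosted damage, then reset after a delay.
; That logic is disconnected and never runs, leaving Boost and Tick empty and BeginPlay only calling its parent.
; The drafted reset also assigns BoostDamage, so damage would stay boosted.
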(event Custom|Boost
  ;[1 1 1] Damage Boost
  ;;[1 0.25 0] Do Boosted Damage
)

(event EventTick
  (params (DeltaSeconds :type Float%20%28single-precision%29)))

(event EventBeginPlay
  (|CallParentFunction))

(fn ConstructionScript
  (|CallParentFunction))

(fn IncrementKillCount
  (Math|Integer|IncrementInt (Variables|Boost|GetKillStreak)))