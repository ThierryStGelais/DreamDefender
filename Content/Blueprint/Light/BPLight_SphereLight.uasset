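; Spherical light actor that damages Nightmare enemies entering its hit detection mesh, built on a base light.
; On actor overlap, it confirms the mesh overlap and enemy line of sight, then passes the light's damage value and frequency to the enemy.
; It overrides the base hit detection setup to configure a query-only mesh that starts at zero scale, storing the requested size in VLightConeSize.
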(event EventBeginPlay)

(event EventInitializeHitDetection
  (params (mesh :type Static%20Mesh%20Object%20Reference) (meshRotation :type Rotator) (MeshLocation :type Vector) (coneMeshSize :type Vector) (ConeVisible :type Boolean) (IsOn :type Boolean))
  (bind _hitdetectionmesh (Variables|Default|GetHitDetectionMesh))
  ;[1 1 1] OVERRIDE DE HIT DETECTION DE BASELIGHT
  (Components|StaticMesh|SetStaticMesh _hitdetectionmesh mesh)
  (Transformation|SetRelativeLocationAndRotation _hitdetectionmesh MeshLocation meshRotation false false)
  (Development|SetHiddeninGame _hitdetectionmesh (not ConeVisible) false)
  (Transformation|SetRelativeScale3D _hitdetectionmesh "0, 0, 0")
  (Variables|Default|SetvLightConeSize coneMeshSize)
  (Collision|SetCollisionEnabled _hitdetectionmesh "QueryOnly")
  (Collision|SetCollisionObjectType _hitdetectionmesh "ECC_WorldStatic")
  (Rendering|SetVisibility _hitdetectionmesh IsOn false))

(event EventActorBeginOverlap
  (params (OtherActor :type Actor%20Object%20Reference))
  (if (Collision|IsOverlappingActor (Variables|Default|GetHitDetectionMesh) OtherActor :!class /Script/Engine.PrimitiveComponent)
    (bind _asnightmare_base_class (Utilities|Casting|CastToNightmare_BaseClass OtherActor))
    (bind _returnvalue (Class|BaseLight|GetDamageValue))
    (bind _returnvalue_2 (Class|BaseLight|GetDamageTime))
    (bind _returnvalue_3 (Class|BaseLight|CheckEnemyLineOfSight _asnightmare_base_class))
    (if _returnvalue_3
      (Class|NightmareBaseClass|ReceiveDamage _asnightmare_base_class _returnvalue _returnvalue_2))))

(event EventTick
  (params (DeltaSeconds :type Float%20%28single-precision%29)))

(fn ConstructionScript)