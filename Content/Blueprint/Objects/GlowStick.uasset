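; Thrown glow stick that creates a temporary sphere of light, configured with damage, through a child BPLight_SphereLight actor.
; It triggers on hitting actors with certain name prefixes or after a maximum airtime, playing a sound and growing the sphere and intensity by timeline.
; Tick countdowns then damp its physics velocities and activate explosion particles, and later shrink the light.
; The stick swaps material and destroys itself after a delay.
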(event OnComponentHit(CollisionCapsule)
  (params (OtherActor :type Actor%20Object%20Reference) (OtherComp :type Primitive%20Component%20Object%20Reference) (NormalImpulse :type Vector :default "0, 0, 0") (Hit :type Hit%20Result%20Structure%20%28by%20ref%29))
  (bind _returnvalue (Utilities|GetObjectName OtherActor))
  ;[1 1 1] Vérifie si le stick a atterie sur une object
  (if (Math|Boolean|ORBoolean (Utilities|String|StartsWith _returnvalue "SM_FLOOR") (Utilities|String|StartsWith _returnvalue "SM_TAPI") (Utilities|String|StartsWith _returnvalue "SM_COFFRE") (Utilities|String|StartsWith _returnvalue "SM_CHEVET"))
    (Variables|Default|SetHasLanded true)))

(event EventTick
  (params (DeltaSeconds :type Float%20%28single-precision%29))
  ;[1 1 1] Event tick
  (Variables|Default|SetTimeSinceThrow (+ DeltaSeconds (Variables|Default|GetTimeSinceThrow)))
  (if (or (Variables|Default|GetHasLanded) (> (Variables|Default|GetTimeSinceThrow) (Variables|Default|GetTimeSinceThrowMaximum)))
    (CallFunction|CalculateTimes DeltaSeconds)
    (Utilities|FlowControl|Sequence
      (:then_0
        (Utilities|FlowControl|DoOnce false
          (:Completed
            (Audio|Components|Audio|Play (Variables|Default|GetExplosion%20Sound) 0.0)
            (CallFunction|ActivateStick)
            (bind (_direction _lerpfactormesh _lerpfactorlightint) (Timeline|GrowTimeline Play)
              (:Update
                (CallFunction|GrowSphere _lerpfactormesh _lerpfactorlightint))))))
      (:then_1
        (if (<= (Variables|Default|GetTimeBeforeRotationLock) 0.0)
          (CallFunction|SlowDownStick)
          (Components|Activation|Activate (Variables|Default|GetP_Explosion) false)))
      (:then_2
        (if (<= (Variables|Default|GetTimeBeforeGone) 0.0)
          (Utilities|FlowControl|DoOnce false
            (:Completed
              (bind (_direction_2 _lerpfactormesh_2 _lerpfactorlightint_2) (Timeline|DeGrowTimeline Play)
                (:Update
                  (CallFunction|DeGrowSphere _lerpfactorlightint_2 _lerpfactormesh_2))
                (:Finished
                  (Rendering|Material|SetMaterial (Variables|Default|GetSM_GlowStick) 0 "/Game/Material/M_Glowstick.M_Glowstick")
                  (Utilities|FlowControl|Delay 0 (Variables|Default|GetTimeBeforeGlowStickDisappear))
                  (Actor|DestroyActor))))))))))

(event EventBeginPlay
  (Components|Timeline|SetPlayRate (Variables|Default|GetGrowTimeline) (Variables|Default|GetGrowFactor))
  (Components|Timeline|SetPlayRate (Variables|Default|GetDeGrowTimeline) (Variables|Default|GetDeGrowFactor)))

(event EventActorBeginOverlap
  (params (OtherActor :type Actor%20Object%20Reference)))

(fn ConstructionScript
  (bind _asbplight_sphere_light (Utilities|Casting|CastToBPLight_SphereLight (Variables|/Script/Engine.ChildActorComponent|GetChildActor (Variables|Default|GetBPLight_SphereLight))))
  (Default|InitializeLightSphere _asbplight_sphere_light (Variables|Default|GetIs%20ON) (Variables|Default|GetSm%20Sphere%20Mesh) (Variables|Default|GetF%20Light%20Intensity) (Variables|Default|GetF%20Light%20Damage) (Variables|Default|GetF%20Light%20Damage%20Frequency) (Variables|Default|GetLight%20Color) (Variables|Default|GetSphere%20Mesh%20Size) self (Variables|Default|GetConeVisibleDansLaScene) (Variables|Default|GetMesh%20Position) (Variables|Default|GetMesh%20Rotation) (Variables|Default|GetSphereMaterial)))

(fn ActivateStick
  (if (not (Variables|Default|GethasBeenToggled))
    (bind _asbplight_sphere_light (Utilities|Casting|CastToBPLight_SphereLight (Variables|/Script/Engine.ChildActorComponent|GetChildActor (Variables|Default|GetBPLight_SphereLight))))
    (Class|BaseLight|ToggleLight _asbplight_sphere_light)
    (Rendering|SetVisibility (Variables|/Script/DreamDefender.BaseLight|GetHitDetectionMesh _asbplight_sphere_light) false false)))

(fn CalculateTimes
  (params (tick :type Float%20%28single-precision%29))
  (Variables|Default|SetTimeBeforeGone (- (Variables|Default|GetTimeBeforeGone) tick))
  (Variables|Default|SetTimeBeforeRotationLock (- (Variables|Default|GetTimeBeforeRotationLock) tick)))

(fn SlowDownStick
  (bind _returnvalue (Physics|GetPhysicsLinearVelocity (Variables|Default|GetCollisionCapsule) "None"))
  (Class|PrimitiveComponent|SetAllPhysicsLinearVelocity (Variables|Default|GetCollisionCapsule) (/ _returnvalue 1.5) false)
  (bind _returnvalue_2 (Class|PrimitiveComponent|GetPhysicsAngularVelocity (Variables|Default|GetCollisionCapsule) "None"))
  (Class|PrimitiveComponent|SetPhysicsAngularVelocity (Variables|Default|GetCollisionCapsule) (/ _returnvalue_2 1.5) false "None"))

(fn GrowSphere
  (params (LerpFactorMesh :type Float%20%28single-precision%29) (LerpFactorLightInt :type Float%20%28single-precision%29))
  (bind _asbplight_sphere_light (Utilities|Casting|CastToBPLight_SphereLight (Variables|/Script/Engine.ChildActorComponent|GetChildActor (Variables|Default|GetBPLight_SphereLight))))
  (Transformation|SetWorldScale3D (Variables|/Script/DreamDefender.BaseLight|GetHitDetectionMesh _asbplight_sphere_light) (Math|Vector|Lerp(Vector) "0, 0, 0" (Variables|Default|GetSphere%20Mesh%20Size) LerpFactorMesh))
  (Rendering|Components|Light|SetIntensity (Variables|/Script/DreamDefender.BaseLight|GetPointLight _asbplight_sphere_light) (Math|Float|Lerp 0.0 (Variables|Default|GetF%20Light%20Intensity) LerpFactorLightInt)))

(fn DeGrowSphere
  (params (IntensityFactor :type Float%20%28single-precision%29) (SphereFactor :type Float%20%28single-precision%29))
  (bind _asbplight_sphere_light (Utilities|Casting|CastToBPLight_SphereLight (Variables|/Script/Engine.ChildActorComponent|GetChildActor (Variables|Default|GetBPLight_SphereLight))))
  (Transformation|SetWorldScale3D (Variables|/Script/DreamDefender.BaseLight|GetHitDetectionMesh _asbplight_sphere_light) (Math|Vector|Lerp(Vector) (Variables|Default|GetSphere%20Mesh%20Size) "0, 0, 0" SphereFactor))
  (Rendering|Components|Light|SetIntensity (Variables|/Script/DreamDefender.BaseLight|GetPointLight _asbplight_sphere_light) (Math|Float|Lerp (Variables|Default|GetF%20Light%20Intensity) 0.0 IntensityFactor))
  (Rendering|SetVisibility (Variables|/Script/DreamDefender.BaseLight|GetPointLight _asbplight_sphere_light) (> (Variables|/Script/Engine.LightComponentBase|GetIntensity (Variables|/Script/DreamDefender.BaseLight|GetPointLight _asbplight_sphere_light)) 0.0) false))