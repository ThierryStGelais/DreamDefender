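; LittleGirl is the sleeping girl whose health nightmares drain; at zero, she notifies GameModeDD that she wakes up.
; Health starts at BaseHealth in the construction script, and TakeDamage lowers it, then plays Creep- or Muncher-specific attack feedback if she survives.
; UpdateZNumbers compares the health fraction to ZPopValue thresholds, switching off Z indicators on BP_Life as health falls.
; The event graph holds only an unconnected chain of delayed test damage.
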(event EventBeginPlay)

(event EventActorBeginOverlap
  (params (OtherActor :type Actor%20Object%20Reference)))

(event EventTick
  (params (DeltaSeconds :type Float%20%28single-precision%29)))

(fn ConstructionScript
  (CallFunction|SetCurrentHealth (Variables|Default|GetBase%20Health)))

(fn GetCurrentHealth
  (return (Variables|Default|GetHealth)))

(fn SetCurrentHealth
  (params (Health :type Float%20%28single-precision%29))
  (Variables|Default|SetHealth Health))

(fn TakeDamage
  (params (Damage :type Float%20%28single-precision%29) (NightmareActor :type Actor%20Object%20Reference))
  (bind _health (CallFunction|GetCurrentHealth))
  (bind _attackcreep (Variables|Default|GetAttackCreep))
  (bind _attackmuncher (Variables|Default|GetAttackMuncher))
  (bind _returnvalue (<= _health 0.0))
  (CallFunction|SetCurrentHealth (- _health Damage))
  (CallFunction|UpdateZNumbers)
  (Utilities|Casting|CastToNightmare_Creep NightmareActor
    (:then
      (if _returnvalue
        (CallFunction|Die)
        (elif (not (Audio|Components|Audio|IsPlaying _attackcreep))
          (Audio|Components|Audio|Play _attackcreep 0.0))))
    (:CastFailed
      (Utilities|Casting|CastToNightmare_Muncher NightmareActor)
      (if _returnvalue
        (CallFunction|Die)
        (elif (not (Audio|Components|Audio|IsPlaying _attackmuncher))
          (Audio|Components|Audio|Play _attackmuncher 0.0))))))

(fn Die
  (bind _asgame_mode_dd (Utilities|Casting|CastToGameModeDD (Game|GetGameMode)))
  (Default|EventLittleGirlWakeup _asgame_mode_dd))

(fn UpdateZNumbers
  (bind _znumber (LocalVariables|GetZnumber))
  (while (and (<= (CallFunction|GetHealthPercentage) (Utilities|Array|Get(acopy) (Variables|Default|GetZPopValue) _znumber)) (>= _znumber 0))
    ;[1 1 1] Verifie si le z a déja été tué
    (bind _outactors (Actor|GetAllActorsOfClass 0 "/Game/Blueprint/BP_Life.BP_Life_C"))
    (if (Default|GetZisDead (Utilities|Array|Get(acopy) _outactors) (LocalVariables|GetZnumber))
      _
      (else
        ;[1 1 1] Ferme le Z si il ne l'est pas déja et décremente znumber
        (Default|TurnOffZ _outactors (LocalVariables|GetZnumber))))
    (Math|Integer|DecrementInt (LocalVariables|GetZnumber))))

(fn GetHealthPercentage
  (return (/ (Variables|Default|GetHealth) (Variables|Default|GetBase%20Health))))