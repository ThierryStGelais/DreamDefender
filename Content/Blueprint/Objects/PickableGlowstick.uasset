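; Pickable glowstick that adds one to the player's glowstick count on contact, then plays a pickup sound and destroys itself.
; Pickup only succeeds while the ThirdPersonCharacter's current count is below its maximum.
; BeginPlay handles a player already overlapping the actor when play begins for it.
; ActorBeginOverlap stores an entering character and runs the same capacity check through CheckOverlapWithGlowStick.
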(event Custom|CheckOverlapWithGlowStick
  ;[1 1 1] Au cas où on à l'inventaire plein et qu'on lance un glowstick
  (bind _asthird_person_character (Utilities|Casting|CastToThirdPersonCharacter (Variables|Default|GetPlayer)))
  (bind (_current _max) (Default|GetGlowStickNumbers _asthird_person_character))
  (if (< _current _max)
    (Default|IncrementGlowStickNumber _asthird_person_character)
    (Audio|PlaySoundatLocation 0 "/Game/Audio/Sound/S_Pickup.S_Pickup" (Transformation|GetActorLocation self))
    (Actor|DestroyActor)))

(event EventBeginPlay
  (bind _returnvalue (Game|GetPlayerCharacter 0))
  (if (Collision|IsOverlappingActor _returnvalue :!class /Script/Engine.Actor)
    (bind _asthird_person_character (Utilities|Casting|CastToThirdPersonCharacter _returnvalue))
    (bind (_current _max) (Default|GetGlowStickNumbers _asthird_person_character))
    (if (< _current _max)
      (Default|IncrementGlowStickNumber _asthird_person_character)
      (Audio|PlaySoundatLocation 0 "/Game/Audio/Sound/S_Pickup.S_Pickup" (Transformation|GetActorLocation self))
      (Actor|DestroyActor))))

(event EventActorBeginOverlap
  (params (OtherActor :type Actor%20Object%20Reference))
  ;[1 1 1] Au cas où on à l'inventaire plein et qu'on lance un glowstick
  (bind _asthird_person_character (Utilities|Casting|CastToThirdPersonCharacter OtherActor))
  (Variables|Default|SetPlayer _asthird_person_character)
  (CallFunction|CheckOverlapwithGlowStick))

(fn ConstructionScript)