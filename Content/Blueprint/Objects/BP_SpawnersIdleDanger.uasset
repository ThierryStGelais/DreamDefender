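; BP_SpawnersIdleDanger is a short-lived actor that plays an idle spawner effect, PSpawnerIdle, for the length of a preparation phase.
; On BeginPlay, a set ActivationTime delays the effect, which then runs for the actor's own PrepTime.
; Otherwise it starts immediately and runs for the PreparationTime read from GameModeDD.
; In both cases it deactivates the effect, then destroys itself after a fixed grace delay.
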(event EventBeginPlay
  (if (Variables|Default|GetActivationTime?)
    (Utilities|FlowControl|Delay (Variables|Default|GetActivationTime))
    (Components|Activation|Activate (Variables|Default|GetP_SpawnerIdle) false)
    (Utilities|FlowControl|Delay (Variables|SetTime|GetPrep%20Time))
    (Components|Activation|Deactivate (Variables|Default|GetP_SpawnerIdle))
    (Utilities|FlowControl|Delay 1e+01)
    (Actor|DestroyActor)
    (else
      (bind _asgame_mode_dd (Utilities|Casting|CastToGameModeDD (Game|GetGameMode)))
      (Components|Activation|Activate (Variables|Default|GetP_SpawnerIdle) false)
      (Utilities|FlowControl|Delay (Variables|/Game/Blueprint/Gameloop/GameModeDD.GameModeDD_C|GetPreparationTime _asgame_mode_dd))
      (Components|Activation|Deactivate (Variables|Default|GetP_SpawnerIdle))
      (Utilities|FlowControl|Delay 1e+01)
      (Actor|DestroyActor))))

(fn ConstructionScript)