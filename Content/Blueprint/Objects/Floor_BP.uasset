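; Floor actor Blueprint that applies a Ripple material to its floor mesh as a dynamic instance.
; The construction script creates the dynamic material on element 0 of the Floor component and stores it in DynamicMat.
; Tick runs through a one-second Delay, then prints each scalar parameter name and value of that material, apparently as debug output.
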(event EventBeginPlay)

(event EventActorBeginOverlap
  (params (OtherActor :type Actor%20Object%20Reference)))

(event EventTick
  (params (DeltaSeconds :type Float%20%28single-precision%29))
  (Utilities|FlowControl|Delay 1.0)
  (for _array_element (Variables|/Script/Engine.MaterialInstance|GetScalarParameterValues (Variables|Default|GetDynamicMat))
    (Development|PrintString (Utilities|String|ToString(Name) (.ParameterName (Utilities|Struct|BreakScalarParameterValue _array_element))) false)
    (Development|PrintString (Utilities|String|ToString(Float) (.ParameterValue (Utilities|Struct|BreakScalarParameterValue _array_element))) false)))

(fn ConstructionScript
  (bind _returnvalue (Rendering|Material|CreateDynamicMaterialInstance (Variables|Default|GetFloor) 0 "/Game/Material/Ripple.Ripple" :!class /Script/Engine.PrimitiveComponent))
  (Variables|Default|SetDynamicMat _returnvalue))