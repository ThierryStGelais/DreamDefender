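; Time system Blueprint that runs a timed night-to-day transition when the day/night cycle begins.
; A dynamic sky material receives the total duration, while a skeletal mesh animation moves socket-attached sun and moon lights after prep time.
; Delays at fractions of that duration trigger timelines for light intensities and duration-scaled day, then night, post-process blends.
; Construction can remove either post-process component, and functions toggle each.
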(event Custom|OnBeginDayNightCycle
  (bind _sk_moon_sun (Variables|Default|GetSK_Moon_Sun))
  (bind _preptime__seconds_ (Variables|GameDuration|GetPrepTime%20%28Seconds%29))
  (bind _sunlight (Variables|Default|GetSunLight))
  (bind _time__seconds_ (Variables|GameDuration|GetTime_%28Seconds%29))
  (bind _returnvalue (+ _time__seconds_ _preptime__seconds_))
  (bind _returnvalue_2 (/ 15.0 _returnvalue))
  ;[1 1 1] Night_2_Day_Start
  (Utilities|FlowControl|Sequence
    (:then_0
      (bind _returnvalue_3 (Rendering|Material|CreateDynamicMaterialInstance (Variables|Default|GetSky) 0 "/Game/Material/M_Night2Day_Sky.M_Night2Day_Sky" :!class /Script/Engine.PrimitiveComponent))
      (Rendering|Material|SetScalarParameterValue _returnvalue_3 "Run_Time_(Seconds)" _returnvalue :!class /Script/Engine.MaterialInstanceDynamic))
    (:then_1
      (Utilities|FlowControl|Delay 0 _preptime__seconds_)
      (Components|Animation|PlayAnimation _sk_moon_sun "/Game/Assets/SK_Moon_Sun_Anim.SK_Moon_Sun_Anim" false)
      (Components|Timeline|SetPlayRate _sk_moon_sun (/ (Components|Animation|GetPlayRate _sk_moon_sun) _time__seconds_))
      (Utilities|FlowControl|Delay 0 _time__seconds_)
      ;;[0 0.0966 1] GAME_OVER
      (Rendering|Material|SetScalarParameterValue _returnvalue_3 "Is_Day? (1=YES // 0=NO)" 1.0 :!class /Script/Engine.MaterialInstanceDynamic))
    (:then_2
      ;;[1 1 1] Lights_Intentisty_CTRL
      (Rendering|Components|Light|SetIntensity _sunlight 0.0)
      (Utilities|FlowControl|Delay 0 (/ _returnvalue 1.4))
      (bind _newtrack_0 (Timeline|Timeline_2 PlayFromStart)
        (:Update
          (Rendering|Components|Light|SetIntensity _sunlight _newtrack_0))))
    (:then_3
      (Utilities|FlowControl|Delay 0 (* _returnvalue 0.85))
      (bind _newtrack_0_2 (Timeline|intensity_drop PlayFromStart)
        (:Update
          (Rendering|Components|Light|SetIntensity (Variables|Default|GetMoonLight) _newtrack_0_2))))
    (:then_4
      ;;[0.69 0.03843 0] Set_DayPP_Off
      (Variables|/Script/Engine.PostProcessComponent|SetBlendWeight (Variables|Default|GetPostProcess_Day) 0.0))
    (:then_5
      (Utilities|FlowControl|Delay 0 (* _returnvalue 0.73))
      ;;[0.69 0.03843 0] PP_Blend_(FML)
      (Components|Timeline|SetPlayRate (Variables|Default|GetTimeline_0) _returnvalue_2)
      (bind _newtrack_0_3 (Timeline|Timeline_0 PlayFromStart)
        (:Update
          (Variables|/Script/Engine.PostProcessComponent|SetBlendWeight (Variables|Default|GetPostProcess_Day) _newtrack_0_3))
        (:Finished
          (Components|Timeline|SetPlayRate (Variables|Default|GetTimeline_1) (/ _returnvalue_2 5.0))
          (bind _newtrack_0_4 (Timeline|Timeline_1 PlayFromStart)
            (:Update
              (Variables|/Script/Engine.PostProcessComponent|SetBlendWeight (Variables|Default|GetPostProcess) _newtrack_0_4))))))))

(fn ConstructionScript
  (Utilities|FlowControl|Sequence
    (:then_0
      (Class|SceneComponent|Attachto (Variables|Default|GetMoonLight) (Variables|Default|GetSK_Moon_Sun) "MoonSocket" "KeepWorldPosition" true)
      (Class|SceneComponent|Attachto (Variables|Default|GetSunLight) (Variables|Default|GetSK_Moon_Sun) "SunSocket" "KeepWorldPosition" true))
    (:then_1
      (if (Variables|PostProcessControl|GetSet_PP_Day_Off)
        (Components|DestroyComponent (Variables|Default|GetPostProcess_Day))))
    (:then_2
      (if (Variables|PostProcessControl|GetSet_PP_Night_Off)
        (Components|DestroyComponent (Variables|Default|GetPostProcess))))))

(fn TogglePostProcessDay
  (Variables|/Script/Engine.PostProcessComponent|SetbEnabled (Variables|Default|GetPostProcess_Day) (not (Variables|/Script/Engine.PostProcessComponent|GetbEnabled (Variables|Default|GetPostProcess_Day)))))

(fn TogglePostProcessNight
  (Variables|/Script/Engine.PostProcessComponent|SetbEnabled (Variables|Default|GetPostProcess) (not (Variables|/Script/Engine.PostProcessComponent|GetbEnabled (Variables|Default|GetPostProcess)))))