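; BP_Life is a life indicator made of ten Z meshes that disappear as lives are lost.
; TurnOffZ hides the given Z, spawns a death particle, records it in ZIsDead and rumbles the player character.
; Lower indices also switch the first meshes to Attention or Danger materials.
; GetNextZWorldPosition locates the Z before the first dead one, as depletion runs from last to first, defaulting to the tenth.
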(event EventBeginPlay)

(event EventTick
  (params (DeltaSeconds :type Float%20%28single-precision%29)))

(fn ConstructionScript)

(fn TurnOffZ
  (params (Znumber :type Integer))
  (bind _sk_z2 (Variables|Default|GetSK_Z2))
  (switch int Znumber
    (:0
      (Rendering|SetVisibility (Variables|Default|GetSK_Z1) false false)
      ;[1 1 1] Retroaction Z Disparait
      (Effects|SpawnEmitteratLocation 0 "/Game/Particles/P_ZDeath.P_ZDeath" (Transformation|GetSocketLocation (Variables|Default|GetSK_Z1) "P_IdleSocket"))
      (Utilities|Array|SetArrayElem (Variables|Default|GetZIsDead) 0 true)
      (Utilities|FlowControl|Sequence :!label _label
        (:then_0
          ;[1 1 1] Retroaction danger
          (Development|PrintString 0 "Danger" false)
          (Rendering|Material|SetMaterial _sk_z2 0 "/Game/Material/M_ZZZ_Danger.M_ZZZ_Danger"))
        (:then_1
          _))
      ;[1 1 1] Rumble cast to ThirdPersonCharacter
      (bind _asthird_person_character (Utilities|Casting|CastToThirdPersonCharacter (Game|GetPlayerCharacter 0) :!label _label_2))
      (Default|Rumble _asthird_person_character))
    (:1
      (Rendering|SetVisibility _sk_z2 false false)
      (Effects|SpawnEmitteratLocation 0 "/Game/Particles/P_ZDeath.P_ZDeath" (Transformation|GetSocketLocation (Variables|Default|GetSK_Z2) "P_IdleSocket"))
      (Utilities|Array|SetArrayElem (Variables|Default|GetZIsDead) 1 true)
      (goto _label))
    (:2
      (Rendering|SetVisibility (Variables|Default|GetSK_Z3) false false)
      (Effects|SpawnEmitteratLocation 0 "/Game/Particles/P_ZDeath.P_ZDeath" (Transformation|GetSocketLocation (Variables|Default|GetSK_Z3) "P_IdleSocket"))
      (Utilities|Array|SetArrayElem (Variables|Default|GetZIsDead) 2 true)
      (goto _label))
    (:3
      (Rendering|SetVisibility (Variables|Default|GetSK_Z4) false false)
      (Effects|SpawnEmitteratLocation 0 "/Game/Particles/P_ZDeath.P_ZDeath" (Transformation|GetSocketLocation (Variables|Default|GetSK_Z4) "P_IdleSocket") "0, 0,0.000000")
      (Utilities|Array|SetArrayElem (Variables|Default|GetZIsDead) 3 true)
      (Utilities|FlowControl|Sequence :!label _label_3
        (:then_0
          ;[1 1 1] Retroaction attention
          (Development|PrintString 0 "Attention" false)
          (Rendering|Material|SetMaterial _sk_z2 0 "/Game/Material/M_ZZZ_Attention.M_ZZZ_Attention"))
        (:then_1
          (goto _label_2))))
    (:4
      (Rendering|SetVisibility (Variables|Default|GetSK_Z5) false false)
      (Effects|SpawnEmitteratLocation 0 "/Game/Particles/P_ZDeath.P_ZDeath" (Transformation|GetSocketLocation (Variables|Default|GetSK_Z5) "P_IdleSocket"))
      (Utilities|Array|SetArrayElem (Variables|Default|GetZIsDead) 4 true)
      (goto _label_3))
    (:5
      (Rendering|SetVisibility (Variables|Default|GetSK_Z6) false false)
      (Effects|SpawnEmitteratLocation 0 "/Game/Particles/P_ZDeath.P_ZDeath" (Transformation|GetSocketLocation (Variables|Default|GetSK_Z6) "P_IdleSocket"))
      (Utilities|Array|SetArrayElem (Variables|Default|GetZIsDead) 5 true)
      (goto _label_3))
    (:6
      (Rendering|SetVisibility (Variables|Default|GetSK_Z7) false false)
      (Effects|SpawnEmitteratLocation 0 "/Game/Particles/P_ZDeath.P_ZDeath" (Transformation|GetSocketLocation (Variables|Default|GetSK_Z7) "P_IdleSocket"))
      (Utilities|Array|SetArrayElem (Variables|Default|GetZIsDead) 6 true)
      (goto _label_2))
    (:7
      (Rendering|SetVisibility (Variables|Default|GetSK_Z8) false false)
      (Effects|SpawnEmitteratLocation 0 "/Game/Particles/P_ZDeath.P_ZDeath" (Transformation|GetSocketLocation (Variables|Default|GetSK_Z8) "P_IdleSocket"))
      (Utilities|Array|SetArrayElem (Variables|Default|GetZIsDead) 7 true)
      (goto _label_2))
    (:8
      (Rendering|SetVisibility (Variables|Default|GetSK_Z9) false false)
      (Effects|SpawnEmitteratLocation 0 "/Game/Particles/P_ZDeath.P_ZDeath" (Transformation|GetSocketLocation (Variables|Default|GetSK_Z9) "P_IdleSocket") "0, 0,0.000000")
      (Utilities|Array|SetArrayElem (Variables|Default|GetZIsDead) 8 true)
      (goto _label_2))
    (:9
      (Rendering|SetVisibility (Variables|Default|GetSK_Z10) false false)
      (Effects|SpawnEmitteratLocation 0 "/Game/Particles/P_ZDeath.P_ZDeath" (Transformation|GetSocketLocation (Variables|Default|GetSK_Z10) "P_IdleSocket"))
      (Utilities|Array|SetArrayElem (Variables|Default|GetZIsDead) 9 true)
      (goto _label_2))))

(fn GetZisDead
  (params (Znumber :type Integer))
  (return (Utilities|Array|Get(acopy) (Variables|Default|GetZIsDead) Znumber)))

(fn GetNextZWorldPosition
  (bind _zisdead (Variables|Default|GetZIsDead))
  (bind _returnvalue (Utilities|Array|FindItem _zisdead true))
  ;[1 1 1] Si il s'agit du premier Z, on le retourne manuellement comme suivant
  (if (== _returnvalue -1)
    _
    (else
      ;[1 1 1] Si il s'agit du dernier Z, on retourne le premier pour pas que unreal panique
      (if (== _returnvalue 0)
        _
        (else
          ;[1 1 1] Retourne la pos du prochaine z
          (bind _returnvector (CallFunction|SwitchonZNumber (- _returnvalue 1)))
          (return _returnvector)))))
  ;[1 1 1] Retourne la pos du premier Z
  (bind _returnvector_2 (CallFunction|SwitchonZNumber 9))
  (return _returnvector_2))

(fn SwitchonZNumber
  (params (Znumber :type Integer))
  (switch int Znumber
    (:0
      (LocalVariables|SetVector (Transformation|GetWorldLocation (Variables|Default|GetSK_Z1))))
    (:1
      (LocalVariables|SetVector (Transformation|GetWorldLocation (Variables|Default|GetSK_Z2))))
    (:2
      (LocalVariables|SetVector (Transformation|GetWorldLocation (Variables|Default|GetSK_Z3))))
    (:3
      (LocalVariables|SetVector (Transformation|GetWorldLocation (Variables|Default|GetSK_Z4))))
    (:4
      (LocalVariables|SetVector (Transformation|GetWorldLocation (Variables|Default|GetSK_Z5))))
    (:5
      (LocalVariables|SetVector (Transformation|GetWorldLocation (Variables|Default|GetSK_Z6))))
    (:6
      (LocalVariables|SetVector (Transformation|GetWorldLocation (Variables|Default|GetSK_Z7))))
    (:7
      (LocalVariables|SetVector (Transformation|GetWorldLocation (Variables|Default|GetSK_Z8))))
    (:8
      (LocalVariables|SetVector (Transformation|GetWorldLocation (Variables|Default|GetSK_Z9))))
    (:9
      (LocalVariables|SetVector (Transformation|GetWorldLocation (Variables|Default|GetSK_Z10)))))
  (return (LocalVariables|GetVector)))